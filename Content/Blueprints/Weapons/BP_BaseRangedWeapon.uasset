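; BP_BaseRangedWeapon is a base Blueprint for ranged weapons that gates use on available ammunition.
; HasAmmo reports whether AmmoCount is above zero, and CanUseWeapon returns that result as the usability check.
; The construction script only calls its parent implementation.
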(fn `CanUseWeapon`
  (returns (Result :type Boolean))
  (bind _result (`self.HasAmmo`))
  (if _result
    (return true)
    (else
      (return false))))

(fn `HasAmmo`
  (returns (Result :type Boolean))
  (if (> (`self.AmmoCount`) 0.0)
    (return true)
    (else
      (return false))))

(fn `UserConstructionScript`
  (`parent.UserConstructionScript`))