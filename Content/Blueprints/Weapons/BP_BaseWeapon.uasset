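; BP_BaseWeapon is a base weapon Blueprint that provides a skeleton for authority-checked weapon use.
; UseWeapon checks CanUseWeapon before calling AttemptServerUseWeapon, which repeats the check on the authority and prints a debug attack or failure message.
; CanUseWeapon always returns false here, so UseWeapon never reaches the attempt event unless that function is overridden.
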(event `UseWeapon`
  (bind _result (`self.CanUseWeapon`))
  (if _result
    (`self.AttemptServerUseWeapon`)))

(event `AttemptServerUseWeapon`
  (`/Engine/EditorBlueprintResources/ActorMacros.Switch Has Authority`
    (:`Authority`
      (bind _result (`self.CanUseWeapon`))
      (if _result
        (`KismetSystemLibrary.PrintString` "Attack")
        (else
          (`KismetSystemLibrary.PrintString` "Can't Attack"))))))

(fn `CanUseWeapon`
  (returns (Result :type Boolean))
  (return false))

(fn `UserConstructionScript`)