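; BP_LightSaber is a melee weapon owned by BP_Player that drives a two-hit slash combo.
; On authority, the use event sets the player's IsAttacking flag, or SaveAttack if an attack is already running.
; A separate animation event alternates two great sword montages through the player's ComboCounter.
; Fixed damage is applied when an overlap ends, skipping actors that share the saber's instigator controller.
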(event `self.ReceiveBeginPlay`
  (bind _asbp_player (cast `/Game/Blueprints/BP_Player` (`self.GetOwner`)))
  (set `self.Character` _asbp_player))

(event `self.UseWeaponEvent`
  (bind _character (`self.Character`))
  (`/Engine/EditorBlueprintResources/ActorMacros.Switch Has Authority`
    (:`Authority`
      (if (`/Game/Blueprints/BP_Player.isAttacking` _character)
        (set `/Game/Blueprints/BP_Player.SaveAttack` true _character)
        (else
          (set `/Game/Blueprints/BP_Player.isAttacking` true _character))))))

(event `self.WeaponAnimationEvent`
  (`self.WeaponAnimations`))

(event `self.ReceiveActorEndOverlap`
  (params (OtherActor :type "Actor Object Reference"))
  (bind _returnvalue (`self.GetInstigatorController`))
  (if (!= (`self.GetInstigatorController` OtherActor) _returnvalue)
    (`GameplayStatics.ApplyDamage` OtherActor 15.0 _returnvalue self)))

(fn `UserConstructionScript`)

(fn `WeaponAnimations`
  (bind _character (`self.Character`))
  (bind _returnvalue (`SkeletalMeshComponent.GetAnimInstance` (`Character.Mesh` (`self.Character`))))
  (switch `int` (`/Game/Blueprints/BP_Player.ComboCounter` (`self.Character`))
    (:`0`
      (set `/Game/Blueprints/BP_Player.ComboCounter` 1 _character)
      (`AnimInstance.Montage_Play` _returnvalue "/Game/Assets/Animations/GreatSword/Great_sword_Slash_Montage.Great_sword_Slash_Montage" 1.0 "MontageLength" 0.0 true))
    (:`1`
      (set `/Game/Blueprints/BP_Player.ComboCounter` 0 _character)
      (`AnimInstance.Montage_Play` _returnvalue "/Game/Assets/Animations/GreatSword/Great_sword_Slash_2_Montage.Great_sword_Slash_2_Montage" 1.0 "MontageLength" 0.0 true))))