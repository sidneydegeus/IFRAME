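; BP_Rifle is a weapon that fires BP_Bullet projectiles for the BP_Player that owns it.
; Its UseWeaponEvent spawns a bullet only with authority, so projectile creation is server-side.
; The bullet starts at the ProjectileDirection component, shifted by a camera-rotated GunOffset, and faces along the player camera's rotation.
; Spawning nudges the bullet out of collisions, or skips it if no clear spot exists.
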(event `self.UseWeaponEvent`
  (`/Engine/EditorBlueprintResources/ActorMacros.Switch Has Authority`
    (:`Authority`
      (bind _asbp_player (cast `/Game/Blueprints/BP_Player` (`self.GetOwner`)))
      (bind _returnvalue (`SceneComponent.K2_GetComponentRotation` (`/Game/Blueprints/BP_Player.PlayerCamera` _asbp_player)))
      (`|SpawnActorFromClass` "/Game/Blueprints/Ammo/BP_Bullet.BP_Bullet_C" (`KismetMathLibrary.MakeTransform` (+ (`SceneComponent.K2_GetComponentLocation` (`self.ProjectileDirection`)) (`KismetMathLibrary.GreaterGreater_VectorRotator` (`self.GunOffset`) _returnvalue)) _returnvalue) "AdjustIfPossibleButDontSpawnIfColliding" "OverrideRootScale" null null))))

(fn `UserConstructionScript`
  (`parent.UserConstructionScript`))